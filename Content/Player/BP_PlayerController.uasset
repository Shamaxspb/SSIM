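; Player controller Blueprint that handles Enhanced Input for side-to-side movement and jumping.
; IA_Move branches to add movement input along the world right axis or its negation, with debug prints.
; Its comparisons test a constant zero rather than the action value, so neither direction fires as written.
; IA_Jump starts the player character's jump on Started and stops it on Completed.
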(event `EnhancedInput|/Game/Player/Input/IA_Move`
  (params (ActionValue :type "Float (double-precision)") (ElapsedSeconds :type "Float (double-precision)") (TriggeredSeconds :type "Float (double-precision)") (InputAction :type "InputAction Object Reference" :default "/Game/Player/Input/IA_Move.IA_Move"))
  (:`Triggered`
    (`KismetSystemLibrary.PrintString` "Hello" true true (struct :`G` 0.66 :`B` 1.0 :`A` 1.0) 0.1 :!enabledstate Disabled)
    (if (`KismetMathLibrary.NearlyEqual_FloatFloat` 0.0 1.0)
      (`Pawn.AddMovementInput` (`GameplayStatics.GetPlayerPawn` 0) (`KismetMathLibrary.Vector_Right`) 1.0 false)
      (`KismetSystemLibrary.PrintString` "Right" true false (struct :`R` 1.0 :`G` 0.214155 :`B` 0.301729 :`A` 1.0) 0.1)
      (elif (`KismetMathLibrary.NearlyEqual_FloatFloat` 0.0 -1.0)
        (`Pawn.AddMovementInput` (`GameplayStatics.GetPlayerPawn` 0) (`KismetMathLibrary.NegateVector` (`KismetMathLibrary.Vector_Right`)) 1.0 false)
        (`KismetSystemLibrary.PrintString` "Left" true false (struct :`R` 0.508997 :`G` 1.0 :`B` 0.462415 :`A` 1.0) 0.1)))))

(event `EnhancedInput|/Game/Player/Input/IA_Jump`
  (params (ActionValue :type Boolean) (ElapsedSeconds :type "Float (double-precision)") (TriggeredSeconds :type "Float (double-precision)") (InputAction :type "InputAction Object Reference" :default "/Game/Player/Input/IA_Jump.IA_Jump"))
  (bind _returnvalue (`GameplayStatics.GetPlayerCharacter` 0))
  (:`Started`
    (`Character.Jump` _returnvalue))
  (:`Completed`
    (`Character.StopJumping` _returnvalue)))

(fn `UserConstructionScript`)