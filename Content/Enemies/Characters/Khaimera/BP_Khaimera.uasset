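; BP_Khaimera is the Khaimera enemy character Blueprint, set up with an SSIM Ability System Component from the Gameplay Ability System.
; BeginPlay and the construction script are empty, so its graphs add no active behavior.
; Disconnected debug nodes remain that would print all abilities, delay briefly, or try activating the combat attack ability by tag and print success or failure.
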(event `self.ReceiveBeginPlay`)

(fn `UserConstructionScript`)